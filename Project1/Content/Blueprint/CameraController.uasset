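; Camera controller Blueprint that switches the player's view among an array of cameras and opens the pause menu.
; On BeginPlay it views the first camera, adds the HUD widget and hides the cursor with game-only input.
; Left and right mouse clicks step forward and back through the cameras, wrapping at the ends.
; P pauses the game, adds the pause widget and shows the cursor, though input stays game-only.
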(event `self.ReceiveBeginPlay`
  (bind _returnvalue (`GameplayStatics.GetPlayerController` 0))
  (bind _output_get (set `self.Index` 0))
  (`PlayerController.SetViewTargetWithBlend` (`GameplayStatics.GetPlayerController` 0) (`|GetArrayItem` (`self.Cameras`) _output_get) 0.0 "VTBlend_Linear" 0.0 false)
  (bind _returnvalue_2 (`|CreateWidget` "/Game/UI/MyHUD_WBP.MyHUD_WBP_C"))
  (`UserWidget.AddToViewport` _returnvalue_2 0)
  (set `PlayerController.bShowMouseCursor` false _returnvalue)
  (`WidgetBlueprintLibrary.SetInputMode_GameOnly` _returnvalue))

(event `Key|LeftMouseButton`
  (params (Key :type "Key Structure"))
  (:`Pressed`
    (bind _result (`/Engine/EditorBlueprintResources/StandardMacros.IncrementInt` (`self.Index`))
      (:`  `
        (if (not (`KismetArrayLibrary.Array_IsValidIndex` (`self.Cameras`) _result))
          (set `self.Index` 0))
        (`PlayerController.SetViewTargetWithBlend` (`GameplayStatics.GetPlayerController` 0) (`|GetArrayItem` (`self.Cameras`) (`self.Index`)) 0.0 "VTBlend_Linear" 0.0 false)))))

(event `Key|RightMouseButton`
  (params (Key :type "Key Structure"))
  (bind _cameras (`self.Cameras`))
  (:`Pressed`
    (bind _result (`/Engine/EditorBlueprintResources/StandardMacros.DecrementInt` (`self.Index`))
      (:`  `
        (if (not (`KismetArrayLibrary.Array_IsValidIndex` _cameras _result))
          (set `self.Index` (`KismetArrayLibrary.Array_LastIndex` _cameras)))
        (`PlayerController.SetViewTargetWithBlend` (`GameplayStatics.GetPlayerController` 0) (`|GetArrayItem` (`self.Cameras`) (`self.Index`)) 0.0 "VTBlend_Linear" 0.0 false)))))

(event `Key|P`
  (params (Key :type "Key Structure"))
  (bind _returnvalue (`GameplayStatics.GetPlayerController` 0))
  (:`Pressed`
    (`GameplayStatics.SetGamePaused` true)
    (bind _returnvalue_2 (`|CreateWidget` "/Game/UI/PauseMenu_WBP.PauseMenu_WBP_C"))
    (`UserWidget.AddToViewport` _returnvalue_2 0)
    (set `PlayerController.bShowMouseCursor` true _returnvalue)
    (`WidgetBlueprintLibrary.SetInputMode_GameOnly` _returnvalue)))