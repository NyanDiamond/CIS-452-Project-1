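; MyCharacter_BP is a player character Blueprint with basic walking, turning, jumping and sprinting.
; Axis inputs move it along its forward vector and yaw the controller, scaled by speed variables set on BeginPlay and frame delta time.
; Holding Left Shift sprints by doubling WalkSpeed and halving it on release, which scales the movement input value rather than changing the movement component's max speed.
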(event `self.ReceiveBeginPlay`
  (set `self.Walk Speed` 100.0)
  (set `self.Turn Speed` 75.0))

(event `InputAction|Jumping`
  (params (Key :type "Key Structure"))
  (:`Pressed`
    (`self.Jump`)))

(event `InputAxis|CharForward`
  (params (AxisValue :type "Float (single-precision)"))
  (`self.AddMovementInput` (* (`self.GetActorForwardVector`) (* (`self.Walk Speed`) (`GameplayStatics.GetWorldDeltaSeconds`) AxisValue))))

(event `InputAxis|CharTurn`
  (params (AxisValue :type "Float (single-precision)"))
  (`self.AddControllerYawInput` (* AxisValue (`GameplayStatics.GetWorldDeltaSeconds`) (`self.Turn Speed`))))

(event `Key|LeftShift`
  (params (Key :type "Key Structure"))
  (:`Pressed`
    (set `self.Walk Speed` (* (`self.Walk Speed`) 2.0)))
  (:`Released`
    (set `self.Walk Speed` (* (`self.Walk Speed`) 0.5))))

(fn `UserConstructionScript`)